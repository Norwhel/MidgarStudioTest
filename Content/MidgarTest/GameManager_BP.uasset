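; GameManager_BP runs a turn-based fight between a player team and an enemy team, from start to end.
; On BeginPlay it finds the TurnManager_BP in the level, passes it both fighter lists, then starts the fight after a short delay.
; When a character dies, it checks whether that whole side is dead and, if so, notifies the player controller and turn manager to end the game.
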(event EventBeginPlay
  ;[1 1 1] BeginPlay : initialize and starts the fight.
  (bind _outactors (Actor|GetAllActorsOfClass "/Game/MidgarTest/TurnManager_BP.TurnManager_BP_C"))
  (bind _output_get (Variables|Default|SetTurnManagerRef (Utilities|Array|Get(acopy) _outactors)))
  (Default|SetFightersList _output_get (Variables|Default|GetEnemyList) (Variables|Default|GetPlayerCharatersList))
  (Utilities|FlowControl|Delay 0.2)
  (Class|TurnManager|StartFight _output_get))

(fn ConstructionScript)

(fn CheckEndGameCondition
  (params (DeadCharacter :type Character%20BP%20Object%20Reference))
  ;[1 1 1] Called when a character dies. Check if the other characters on his side are dead too. If it's the case, returns true.
  (switch Utilities|FlowControl|Switch|SwitchonTeamSides_Enum (Variables|/Game/MidgarTest/Character_BP.Character_BP_C|GetTeamSide DeadCharacter)
    (:NewEnumerator0
      (for _array_element (Variables|Default|GetEnemyList)
        (if (not (Variables|/Script/testMidgar.TBTCharacter|Getdead _array_element))
          (return false))))
    (:NewEnumerator1
      (for _array_element_2 (Variables|Default|GetPlayerCharatersList)
        (if (not (Variables|/Script/testMidgar.TBTCharacter|Getdead _array_element_2))
          (return false)))))
  (return true))

(fn CheckEndGame
  (params (DeadCharacter :type Character%20BP%20Object%20Reference))
  ;[1 1 1] Called when a character dies. Check if conditions are met to end the game and call end game if ok.
  (bind _condition (CallFunction|CheckEndGameCondition DeadCharacter))
  (if _condition
    (CallFunction|CallEndGame (Variables|/Game/MidgarTest/Character_BP.Character_BP_C|GetTeamSide DeadCharacter))))

(fn CallEndGame
  (params (DefeatSide :type TeamSides_Enum%20Enum :default "NewEnumerator0"))
  ;[1 1 1] Called when game ended, notifies Turn Manager and Player Controller to trigger their respective end game behavior.
  (bind _asplayer_controller (Utilities|Casting|CastToPlayerController (Game|GetPlayerController 0)))
  (Default|EndGame _asplayer_controller DefeatSide)
  (Class|TurnManager|EndGame (Variables|Default|GetTurnManagerRef)))